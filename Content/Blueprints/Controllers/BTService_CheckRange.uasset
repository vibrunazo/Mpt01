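; Behavior tree service that checks on each AI tick whether the controlled pawn is within attack range of its target.
; It caches the blackboard's target actor as a CharBase, reads AttackRange from EnemyController_Basic, and compares it with the distance between pawn and target.
; Helper graphs split up these steps; being in range only prints a debug string, with no blackboard write.
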(event `self.ReceiveTickAI`
  (params (OwnerController :type "AIController Object Reference") (ControlledPawn :type "Pawn Object Reference") (DeltaSeconds :type "Float (single-precision)"))
  (`|ExecutionSequence`
    (:`then_0`
      (bind _aschar_base (cast `/Game/Blueprints/Chars/CharBase` (`BlackboardComponent.GetValueAsObject` (`AIBlueprintHelperLibrary.GetBlackboard` ControlledPawn) (`self.ActorKeyName`))))
      (set `self.TargetActorRef` _aschar_base))
    (:`then_1`
      (bind _asenemy_controller_basic (cast `/Game/Blueprints/Controllers/EnemyController_Basic` OwnerController)))
    (:`then_2`
      (if (<= (`KismetMathLibrary.VSize` (- (`Actor.K2_GetActorLocation` ControlledPawn) (`Actor.K2_GetActorLocation` (`self.TargetActorRef`)))) (`/Game/Blueprints/Controllers/EnemyController_Basic.AttackRange` _asenemy_controller_basic))
        (`KismetSystemLibrary.PrintString` "In Range")))))