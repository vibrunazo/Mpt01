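; Behavior tree service that tells a basic enemy to attack when its blackboard target is within attack range.
; Each AI tick caches the controller and pawn, then reads the target as a CharBase from a blackboard key.
; It compares the distance between the two actors with the EnemyController_Basic attack range.
; When in range, it prints a debug message and calls OrderToAttack on that controller.
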(event `self.ReceiveTickAI`
  (params (OwnerController :type "AIController Object Reference") (ControlledPawn :type "Pawn Object Reference") (DeltaSeconds :type "Float (single-precision)"))
  (`|ExecutionSequence`
    (:`then_0`
      (set `self.ControllerRef` OwnerController))
    (:`then_1`
      (set `self.SelfActorRef` ControlledPawn))
    (:`then_2`
      (bind _aschar_base (cast `/Game/Blueprints/Chars/CharBase` (`BlackboardComponent.GetValueAsObject` (`AIBlueprintHelperLibrary.GetBlackboard` ControlledPawn) (`self.ActorKeyName`))))
      (set `self.TargetActorRef` _aschar_base)
      (`|ExecutionSequence`
        (:`then_0`
          (bind _asenemy_controller_basic (cast `/Game/Blueprints/Controllers/EnemyController_Basic` (`self.ControllerRef`))))
        (:`then_1`
          (if (<= (`KismetMathLibrary.VSize` (- (`Actor.K2_GetActorLocation` (`self.SelfActorRef`)) (`Actor.K2_GetActorLocation` (`self.TargetActorRef`)))) (`/Game/Blueprints/Controllers/EnemyController_Basic.AttackRange` _asenemy_controller_basic))
            (`KismetSystemLibrary.PrintString` "In Range")
            (bind _asenemy_controller_basic_2 (cast `/Game/Blueprints/Controllers/EnemyController_Basic` (`self.ControllerRef`)))
            (`/Game/Blueprints/Controllers/EnemyController_Basic.Order To Attack` _asenemy_controller_basic_2)))))))