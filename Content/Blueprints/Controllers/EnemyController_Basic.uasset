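; Basic enemy AI controller that runs BT_Basic on possess and feeds it a target from AI perception.
; While CanFollow is set, perception updates lock onto an opposing-team CharBase, storing it in the blackboard and clearing CanFollow.
; An update lacking the current target clears it from the blackboard, but CanFollow is only re-enabled on possess.
; Debug strings print candidate names and target loss.
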(event `self.OnPossess`
  (params (PossessedPawn :type "Pawn Object Reference"))
  (`self.RunBehaviorTree` "/Game/Blueprints/Controllers/BT_Basic.BT_Basic")
  (`BlackboardComponent.SetValueAsObject` (`AIBlueprintHelperLibrary.GetBlackboard` null) (`self.BBCharKeyName`) null)
  (set `self.canFollow` true))

(event `self.ReceiveBeginPlay`
  (`parent.ReceiveBeginPlay`))

(event `self.ReceiveTick`
  (params (DeltaSeconds :type "Float (single-precision)")))

(event `self.AIPerception.OnPerceptionUpdated`
  (params (UpdatedActors :type "Array of Actor Object Reference"))
  (if (`self.canFollow`)
    (set `self.hasTarget` false)
    (for _array_element UpdatedActors
      (`KismetSystemLibrary.PrintString` (`KismetSystemLibrary.GetDisplayName` _array_element))
      (bind _aschar_base (cast `/Game/Blueprints/Chars/CharBase` _array_element))
      (bind _aschar_base_2 (cast `/Game/Blueprints/Chars/CharBase` (`self.K2_GetPawn`)))
      (if (!= (`/Game/Blueprints/Chars/CharBase.team` _aschar_base) (`/Game/Blueprints/Chars/CharBase.team` _aschar_base_2))
        (`BlackboardComponent.SetValueAsObject` (`AIBlueprintHelperLibrary.GetBlackboard` null) (`self.BBCharKeyName`) _aschar_base)
        (set `self.CurrentTarget` _aschar_base)
        (set `self.canFollow` false)
        (set `self.hasTarget` true)
        (break))))
  (if (not (`KismetArrayLibrary.Array_Contains` UpdatedActors (`self.CurrentTarget`)))
    (`self.Didn't find anyone in sight`)))

(event `Didn't find anyone in sight`
  (`BlackboardComponent.SetValueAsObject` (`AIBlueprintHelperLibrary.GetBlackboard` null) (`self.BBCharKeyName`) null)
  (set `self.CurrentTarget` null)
  (`KismetSystemLibrary.PrintString` "no one"))

(fn `UserConstructionScript`
  (`parent.UserConstructionScript`))