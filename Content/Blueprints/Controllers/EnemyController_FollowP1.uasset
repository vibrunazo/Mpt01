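; Enemy AI controller that makes its pawn chase player one's character.
; BeginPlay caches the first player character, cast to CharBase, as the move target.
; A custom event issues an AI MoveTo toward it immediately, then repeats it on a looping timer, printing debug success or failure.
; Nothing in this graph calls that start event, and an older MoveToActor branch is left disconnected.
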(event `Follow enemy once`
  (`|AIMoveTo` null (0.0 0.0 0.0) (`self.PlayerChar`)
    (:`OnSuccess`
      (`KismetSystemLibrary.PrintString` "Hello"))
    (:`OnFail`
      (`KismetSystemLibrary.PrintString` "FAIL"))))

(event `Start following timer`
  (`self.Follow enemy once`)
  (`KismetSystemLibrary.K2_SetTimerDelegate` (delegate `Follow enemy once`) 2.0 true))

(event `self.ReceiveBeginPlay`
  (`parent.ReceiveBeginPlay`)
  (bind _aschar_base (cast `/Game/Blueprints/Chars/CharBase` (`GameplayStatics.GetPlayerCharacter` 0)))
  (set `self.PlayerChar` _aschar_base))

(fn `UserConstructionScript`
  (`parent.UserConstructionScript`))