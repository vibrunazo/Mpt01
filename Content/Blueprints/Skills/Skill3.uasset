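; Skill3 is a skill Blueprint that fires a Proj2 projectile from the owning character.
; UseSkill sets the Casting flag on the character's anim Blueprint, waits briefly, then spawns the projectile at the ProjectileSpawn transform with the character as Shooter.
; It clears the flag immediately after spawning, so the casting state lasts only for that short delay.
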(event `self.Use Skill`
  (bind _owning_char (`self.Owning Char`))
  (bind _animbp (`/Game/Blueprints/Chars/CharBase.GetAnimBP` _owning_char))
  (set `/Game/Mannequin/Animations/ThirdPerson_AnimBP.casting` true _animbp)
  (`KismetSystemLibrary.Delay` 0.1)
  (`|SpawnActorFromClass` "/Game/Blueprints/Projectiles/Proj2.Proj2_C" (`SceneComponent.K2_GetComponentToWorld` (`/Game/Blueprints/Chars/CharBase.ProjectileSpawn` (`self.Owning Char`))) "Undefined" "OverrideRootScale" null _owning_char)
  (set `/Game/Mannequin/Animations/ThirdPerson_AnimBP.casting` false _animbp))

(fn `UserConstructionScript`
  (`parent.UserConstructionScript`))