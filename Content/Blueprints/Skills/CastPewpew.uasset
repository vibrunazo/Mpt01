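; CastPewpew is a skill that fires a Proj_pewpew projectile from the owning character.
; SkillStart takes the spawn transform from the owner's ProjectileSpawn component, rotated to face the target character when one is valid.
; It raises the Casting flag on the owner's animation Blueprint, waits briefly, spawns the projectile with the owner as Shooter, then clears the flag.
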(event `self.Skill Start`
  (params (`Target Char` :type "/Game/Blueprints/Chars/CharBase Object Reference"))
  (bind _owning_char (`self.Owning Char`))
  (bind _animbp (`/Game/Blueprints/Chars/CharBase.GetAnimBP` _owning_char))
  (bind (_returnvalue_location _returnvalue_rotation _returnvalue_scale) (`KismetMathLibrary.BreakTransform` (`SceneComponent.K2_GetComponentToWorld` (`/Game/Blueprints/Chars/CharBase.ProjectileSpawn` (`self.Owning Char`)))))
  (`/Engine/EditorBlueprintResources/StandardMacros.IsValid` `Target Char`
    (:`Is Valid`
      (bind _output_get (set `self.target location` (`KismetMathLibrary.MakeTransform` _returnvalue_location (`KismetMathLibrary.FindLookAtRotation` _returnvalue_location (`self.K2_GetActorLocation` `Target Char`)) _returnvalue_scale))))
    (:`Is Not Valid`
      (set `self.target location` (`SceneComponent.K2_GetComponentToWorld` (`/Game/Blueprints/Chars/CharBase.ProjectileSpawn` (`self.Owning Char`))))))
  (set `/Game/Mannequin/Animations/ThirdPerson_AnimBP.casting` true _animbp)
  (`KismetSystemLibrary.Delay` 0.1)
  (`|SpawnActorFromClass` "/Game/Blueprints/Projectiles/Proj_pewpew.Proj_pewpew_C" _output_get "Undefined" "OverrideRootScale" null _owning_char)
  (set `/Game/Mannequin/Animations/ThirdPerson_AnimBP.casting` false _animbp))

(fn `UserConstructionScript`
  (`parent.UserConstructionScript`))