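; Punches is a skill Blueprint that gives its owning character a punch attack.
; Starting and ending the skill toggles the Punching flag on the owner's animation Blueprint.
; On BeginPlay it binds to the owner's attack-box-active event, which creates a damaging hit box on the character whenever it fires.
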(event `self.ReceiveBeginPlay`
  (add `/Game/Blueprints/Chars/CharBase.AttackBoxActive` (`self.Owning Char`) (delegate `AttackActive`)))

(event `AttackActive`
  (`/Game/Blueprints/Chars/CharBase.Create HitBox` (`self.Owning Char`) "None" 5.0))

(event `Skill Start`
  (params (`Target Char` :type "/Game/Blueprints/Chars/CharBase Object Reference"))
  (set `/Game/Mannequin/Animations/ThirdPerson_AnimBP.punching` true (`/Game/Blueprints/Chars/CharBase.GetAnimBP` (`self.Owning Char`))))

(event `Skill End`
  (set `/Game/Mannequin/Animations/ThirdPerson_AnimBP.punching` false (`/Game/Blueprints/Chars/CharBase.GetAnimBP` (`self.Owning Char`))))

(fn `UserConstructionScript`
  (`parent.UserConstructionScript`))