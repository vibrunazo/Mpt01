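; Base skill Blueprint that wraps skill activation and deactivation with active-state and cooldown handling.
; BaseSkillStart runs only when usable, marks the skill active and passes the target to SkillStart; BaseSkillEnd runs only when active and calls SkillEnd.
; SkillStart and SkillEnd are empty hooks for specific skills.
; A CooldownStartsOnEnd flag decides whether the Delay-based cooldown lockout begins at start or at end.
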(event `Skill Start`
  (params (`Target Char` :type "/Game/Blueprints/Chars/CharBase Object Reference")))

(event `Base Skill Start`
  (params (`target Char` :type "/Game/Blueprints/Chars/CharBase Object Reference"))
  (if (`self.canbeused`)
    (`|ExecutionSequence`
      (:`then_0`
        (set `self.isActive` true))
      (:`then_1`
        (`self.Skill Start` `target Char`))
      (:`then_2`
        (if (not (`self.cooldownStartsOnEnd`))
          (`|ExecutionSequence`
            (:`then_0`
              (set `self.canbeused` false))
            (:`then_1`
              (`KismetSystemLibrary.Delay` (`self.cooldown`))
              (set `self.canbeused` true))))))))

(event `Base Skill End`
  (if (`self.isActive`)
    (`|ExecutionSequence`
      (:`then_0`
        (set `self.isActive` false))
      (:`then_1`
        (`self.Skill End`))
      (:`then_2`
        (if (`self.cooldownStartsOnEnd`)
          (`|ExecutionSequence`
            (:`then_0`
              (set `self.canbeused` false))
            (:`then_1`
              (`KismetSystemLibrary.Delay` (`self.cooldown`))
              (set `self.canbeused` true))))))))

(event `Skill End`)

(fn `UserConstructionScript`)