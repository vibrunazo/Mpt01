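; Attack is a skill Blueprint that performs a character attack with an animation and a damaging hit box.
; On skill start it asks the owning character's AnimBP to play the configured montage with start, active and recovery timings, passing itself along.
; When the animation reaches its active phase, the owning character creates a hit box at the configured socket with the configured damage.
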(event `self.Skill Start`
  (params (`Target Char` :type "/Game/Blueprints/Chars/CharBase Object Reference"))
  (`/Game/Mannequin/Animations/ThirdPerson_AnimBP.PlayAnim` (`/Game/Blueprints/Chars/CharBase.GetAnimBP` (`self.Owning Char`)) self (`self.AnimMontageToPlay`) (`self.Anim Start Time`) (`self.Anim Active Time`) (`self.Anim Recovery Time`)))

(event `self.Anim is Active`
  (`/Game/Blueprints/Chars/CharBase.Create HitBox` (`self.Owning Char`) (`self.Hit Socket Name`) (`self.damage`)))

(fn `UserConstructionScript`
  (`parent.UserConstructionScript`))