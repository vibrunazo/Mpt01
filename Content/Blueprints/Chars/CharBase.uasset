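; Base character with health, targeted skills and melee hitboxes.
; Skill slots start and stop skill actors, passing the current target or, if none is valid, the first character overlapping a cone.
; Hitbox actors attach to a given or default hand socket.
; Damage updates the health bar widget; on death, any controller possesses a temporary pawn, then after a short delay repossesses the character with reset stats, updating the camera at each switch.
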(event `self.ReceiveBeginPlay`
  (bind _ashealth (cast `/Game/UI/Health` (`WidgetComponent.GetUserWidgetObject` (`self.HealthBar`))))
  (set `self.HealthWidget` _ashealth)
  (`self.Initialize Char Stats`))

(event `Initialize Char Stats`
  (set `self.Health` 100.0)
  (set `/Game/UI/Health.health` (`self.Health`) (`self.HealthWidget`))
  (set `self.alive` true))

(event `Start Using Skill`
  (params (`skill index` :type Integer))
  (bind _item (`KismetArrayLibrary.Array_Get` (`self.Skill List`) `skill index`))
  (`/Engine/EditorBlueprintResources/StandardMacros.IsValid` _item
    (:`Is Valid`
      (bind _target_char (`self.GetNewTarget`))
      (bind _output_get (set `self.CurrentTarget` _target_char))
      (`/Game/Blueprints/Skills/Skill.Base Skill Start` _item _output_get))))

(event `Stop Using Skill`
  (params (`Skill Index` :type Integer))
  (bind _item (`KismetArrayLibrary.Array_Get` (`self.Skill List`) `Skill Index`))
  (`/Engine/EditorBlueprintResources/StandardMacros.IsValid` _item
    (:`Is Valid`
      (`/Game/Blueprints/Skills/Skill.Base Skill End` _item))))

(event `Die`
  (bind _returnvalue (`self.GetController`))
  (set `self.alive` false)
  (bind _returnvalue_2 (`|SpawnActorFromClass` "/Game/Blueprints/StarterPawn.StarterPawn_C" (`self.GetTransform`) "Undefined" "OverrideRootScale"))
  (`/Engine/EditorBlueprintResources/StandardMacros.IsValid` _returnvalue
    (:`Is Valid`
      (bind _output_get (set `self.mycontroller` _returnvalue))
      (`Controller.Possess` _output_get _returnvalue_2)
      (`self.UpdateCamera`)
      (`KismetSystemLibrary.Delay` 2.0)
      (`self.Revive`))))

(event `Take Damage`
  (params (Damage :type "Float (double-precision)"))
  (if (`self.alive`)
    (bind _output_get (set `self.Health` (`KismetMathLibrary.FMax` (- (`self.Health`) Damage) 0.0)))
    (bind _output_get_2 (set `/Game/UI/Health.health` _output_get (`self.HealthWidget`)))
    (if (<= _output_get_2 0.0)
      (`self.Die`))))

(event `Revive`
  (`Controller.Possess` (`self.mycontroller`) self)
  (`self.K2_DestroyActor` (stale `Die` _returnvalue_2))
  (`self.Initialize Char Stats`)
  (`self.UpdateCamera`))

(event `PositionAttackBoxOnLeftHand`
  (set `self.AttackSocketName` "hand_lSocket"))

(event `PositionAttackBoxOnRightHand`
  (set `self.AttackSocketName` "hand_rSocket"))

(event `Create HitBox`
  (params (SocketName :type Name :default "None") (Damage :type "Float (double-precision)"))
  (bind _returnvalue (`|SpawnActorFromClass` "/Game/Blueprints/AttackHitBox.AttackHitBox_C" (`self.GetTransform`) "Undefined" "OverrideRootScale" null self Damage))
  (`self.K2_AttachToComponent` _returnvalue (`self.Mesh`) (select `bool` (== SocketName "None") :`false` SocketName :`true` (`self.AttackSocketName`)) "SnapToTarget" "KeepRelative" "KeepRelative" true))

(fn `CreateSkillFromClass`
  (params (`Skill Name` :type "/Game/Blueprints/Skills/Skill Class Reference"))
  (returns (`New Skill` :type "/Game/Blueprints/Skills/Skill Object Reference"))
  (bind _returnvalue (`|SpawnActorFromClass` `Skill Name` (`self.GetTransform`) "Undefined" "OverrideRootScale" null self))
  (`self.K2_AttachToActor` _returnvalue self "None" "SnapToTarget" "SnapToTarget" "SnapToTarget" true)
  (return _returnvalue))

(fn `FindFirstTarget`
  (returns (`Target Char` :type "/Game/Blueprints/Chars/CharBase Object Reference"))
  (bind _cone (`self.Cone`))
  (bind _outactors (`KismetSystemLibrary.ComponentOverlapActors` _cone (`SceneComponent.K2_GetComponentToWorld` _cone) (`|MakeArray` "ObjectTypeQuery3" :!type "EObjectTypeQuery Enum") "CharBase_C" (`|MakeArray` self :!type "Actor Object Reference")))
  (bind _aschar_base (cast `/Game/Blueprints/Chars/CharBase` (`KismetArrayLibrary.Array_Get` _outactors))
    (:`then`
      (return _aschar_base))
    (:`CastFailed`
      (return null))))

(fn `GetAnimBP`
  (returns (AnimBP :type "/Game/Mannequin/Animations/ThirdPerson_AnimBP Object Reference"))
  (return (cast `/Game/Mannequin/Animations/ThirdPerson_AnimBP` (`SkeletalMeshComponent.GetAnimInstance` (`self.Mesh`)) :!pure true)))

(fn `GetNewTarget`
  (returns (`Target Char` :type "/Game/Blueprints/Chars/CharBase Object Reference"))
  (`/Engine/EditorBlueprintResources/StandardMacros.IsValid` (`self.CurrentTarget`)
    (:`Is Valid`
      (return (`self.CurrentTarget`)))
    (:`Is Not Valid`
      (bind _target_char (`self.FindFirstTarget`))
      (return _target_char))))

(fn `UpdateCamera`
  (`/Game/Blueprints/MPTGameMode.Update Camera` (`self.GetMPTGameMode`)))

(fn `UserConstructionScript`
  (`parent.UserConstructionScript`))